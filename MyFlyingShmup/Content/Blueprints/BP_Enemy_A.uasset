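; BP_Enemy_A is an enemy actor that fires bullets automatically on a repeating timer.
; BeginPlay starts a looping three-second timer that triggers ShootBullet.
; Each trigger plays a sci-fi shot sound and spawns BP_EnemyBullet at the BulletSpawnPoint transform, then repeats both after a one-second delay, producing a two-shot burst.
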(event Custom|ShootBullet
  (Audio|PlaySound2D "/Game/Sci-Fi_Shots_Pack2_Game_Of_Weapons/Cue/SciFi_Shot_P2__160__Cue.SciFi_Shot_P2__160__Cue" 1.0 1.0 0.0 0 0)
  (Game|SpawnActorfromClass "/Game/Blueprints/BP_EnemyBullet.BP_EnemyBullet_C" (Transformation|GetWorldTransform (Variables|Default|GetBulletSpawnPoint)) "Undefined" "MultiplyWithRoot" 0 0)
  (Utilities|FlowControl|Delay 1.0)
  (Audio|PlaySound2D "/Game/Sci-Fi_Shots_Pack2_Game_Of_Weapons/Cue/SciFi_Shot_P2__160__Cue.SciFi_Shot_P2__160__Cue" 1.0 1.0 0.0 0 0)
  (Game|SpawnActorfromClass "/Game/Blueprints/BP_EnemyBullet.BP_EnemyBullet_C" (Transformation|GetWorldTransform (Variables|Default|GetBulletSpawnPoint)) "Undefined" "MultiplyWithRoot" 0 0))

(event EventBeginPlay
  (Utilities|Time|SetTimerbyEvent (delegate Custom|ShootBullet) 3.0 true true))

(fn ConstructionScript)