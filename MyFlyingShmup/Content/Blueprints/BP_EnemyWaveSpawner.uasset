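; Enemy wave spawner actor that spawns timed waves of enemies defined in WaveDataAsset.
; Each wave starts after its initial delay, then loops through its members, delaying before each spawn and passing pickup-drop settings to the spawned enemy.
; The next wave is scheduled once the last member spawns, without waiting for kills.
; After the final wave finishes spawning, it tells the HUD to show the end screen.
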(event Custom|StartWave
  (bind _wavedataasset (Variables|Default|GetWaveDataAsset))
  (bind _currentwaveindex (Variables|Default|GetCurrentWaveIndex))
  (bind _setofwaves (Variables|/Game/FrameWork/PDA_SetOfWaves.PDA_SetOfWaves_C|GetSetOfWaves _wavedataasset))
  (bind _output (Utilities|Array|Get(acopy) _setofwaves _currentwaveindex))
  (bind _output_get (Variables|Default|SetEnemyMemberIndex 0))
  (if (> _output_get (Utilities|Array|LastIndex (.enemymembers _output))) :!label _label
    (CallFunction|NextWave)
    (else
      (Utilities|FlowControl|Delay (.initialspawndelay (Utilities|Array|Get(acopy) (.enemymembers _output) (Variables|Default|GetEnemyMemberIndex))))
      (bind _returnvalue (Game|SpawnActorfromClass (.enemyclass (Utilities|Array|Get(acopy) (.enemymembers _output) (Variables|Default|GetEnemyMemberIndex))) (.spawntransform (Utilities|Array|Get(acopy) (.enemymembers _output) (Variables|Default|GetEnemyMemberIndex))) "AlwaysSpawn" "MultiplyWithRoot" 0 0))
      (Class|BPIMyFlyingShmup|AssignSpawnEnemyProps(Message) _returnvalue (.shoulddroppickup (Utilities|Array|Get(acopy) (.enemymembers _output) (Variables|Default|GetEnemyMemberIndex))) (.pickupclass (Utilities|Array|Get(acopy) (.enemymembers _output) (Variables|Default|GetEnemyMemberIndex))))
      (Math|Integer|IncrementInt (Variables|Default|GetEnemyMemberIndex)
        (:%20%20
          (goto _label))))))

(event Custom|NextWave
  (bind _result (Math|Integer|IncrementInt (Variables|Default|GetCurrentWaveIndex))
    (:%20%20
      (if (Utilities|Array|IsValidIndex (Variables|/Game/FrameWork/PDA_SetOfWaves.PDA_SetOfWaves_C|GetSetOfWaves (stale EventBeginPlay _wavedataasset)) _result)
        (Utilities|Time|SetTimerbyEvent (delegate Custom|StartWave) (.initialwavedelay (Utilities|Array|Get(acopy) (Variables|/Game/FrameWork/PDA_SetOfWaves.PDA_SetOfWaves_C|GetSetOfWaves (stale EventBeginPlay _wavedataasset)) (Variables|Default|GetCurrentWaveIndex))))
        (else
          (Class|BPIMyFlyingShmup|ShowEndScreen(Message) (HUD|GetHUD (Game|GetPlayerController 0)) true))))))

(event EventBeginPlay
  (bind _wavedataasset (Variables|Default|GetWaveDataAsset)
    (:then
      (Utilities|Time|SetTimerbyEvent (delegate Custom|StartWave) (.initialwavedelay (Utilities|Array|Get(acopy) (Variables|/Game/FrameWork/PDA_SetOfWaves.PDA_SetOfWaves_C|GetSetOfWaves _wavedataasset) (Variables|Default|GetCurrentWaveIndex)))))
    (:else)))

(fn ConstructionScript)