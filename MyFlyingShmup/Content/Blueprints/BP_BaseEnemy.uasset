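; Base enemy Blueprint that tracks health, shows it on a widget health bar, and deals damage equal to its MaxHealth to actors it overlaps.
; Non-lethal hits play a sound and briefly flash an overlay material on all static meshes.
; When health equals exactly zero, it triggers camera shake, awards MaxHealth as score, spawns an explosion and an optional spawner-assigned pickup, then destroys itself.
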(event Custom|ApplyDamage
  (params (Damage :type Float%20%28double-precision%29))
  ;[0.15 0.15 0.15 0.5] Set progress Health Bar
  (Variables|Default|SetHealth (- (Variables|Default|GetHealth) Damage))
  (bind _aswbp_enemy_health_bar (Utilities|Casting|CastToWBP_EnemyHealthBar (UserInterface|GetUserWidgetObject (Variables|Default|GetWidget))))
  (Default|SetHealth _aswbp_enemy_health_bar (/ (Variables|Default|GetHealth) (Variables|Default|GetMaxHealth))))

(event EventAssignSpawnEnemyProps
  (params (SpawnPickUpOnDeath :type Boolean) (PickUpTypeToSpawn :type BP%20Base%20Pickup%20Class%20Reference))
  (Variables|Default|SetSpawn%20Pick%20Up%20on%20Death SpawnPickUpOnDeath)
  (Variables|Default|SetPick%20Up%20Type%20to%20Spawn PickUpTypeToSpawn))

(event EventBeginPlay
  (Variables|Default|SetHealth (Variables|Default|GetMaxHealth)))

(event Game|Damage|EventAnyDamage
  (params (Damage :type Float%20%28single-precision%29) (DamageType :type Damage%20Type%20Object%20Reference) (InstigatedBy :type Controller%20Object%20Reference) (DamageCauser :type Actor%20Object%20Reference))
  (CallFunction|ApplyDamage Damage)
  ;[0.15 0.15 0.15 0.5] Check if Enemy's Health is ZERO, If so, start death sequence
  (if (== (Variables|Default|GetHealth) 0.0)
    (Audio|PlaySound2D "/Game/Game_Item/Destruction/Wav/Wav_Destructionsoundsw6_wav.Wav_Destructionsoundsw6_wav" 1.0 1.0 0.0 0 0)
    (Utilities|FlowControl|Sequence
      (:then_0
        (bind _asmy_player_controller (Utilities|Casting|CastTomyPlayerController (Game|GetPlayerController 0)))
        (Default|ApplyCameraShake _asmy_player_controller)
        (Default|AddtoScore _asmy_player_controller (Variables|Default|GetMaxHealth)))
      (:then_1
        (Game|SpawnActorfromClass "/Game/Particles/BP_EnemyDeathExplosion.BP_EnemyDeathExplosion_C" (Math|Transform|MakeTransform (Transformation|GetActorLocation) "0, 0, 0" "1.000000,1.000000,1.000000") "AlwaysSpawn" "MultiplyWithRoot" 0 0)
        (if (Variables|Default|GetSpawn%20Pick%20Up%20on%20Death)
          (Game|SpawnActorfromClass (Variables|Default|GetPick%20Up%20Type%20to%20Spawn) (Transformation|GetActorTransform) "AlwaysSpawn" "MultiplyWithRoot" 0 0)))
      (:then_2
        (Actor|DestroyActor)))
    (else
      (Audio|PlaySound2D "/Game/Sci-Fi_Shots_Pack2_Game_Of_Weapons/Cue/SciFi_Shot_P2__106__Cue.SciFi_Shot_P2__106__Cue" 1.0 1.0 0.0 0 0)
      (for _array_element (Actor|GetComponentsByClass "/Script/Engine.StaticMeshComponent")
        (Rendering|Material|SetOverlayMaterial _array_element "/Game/Materials/MI_DamageFlash.MI_DamageFlash" :!class /Script/Engine.MeshComponent))
      (Utilities|FlowControl|Delay 0.2)
      (for _array_element_2 (Actor|GetComponentsByClass "/Script/Engine.StaticMeshComponent")
        (Rendering|Material|SetOverlayMaterial _array_element_2 0 :!class /Script/Engine.MeshComponent)))))

(event Collision|EventActorBeginOverlap
  (params (OtherActor :type Actor%20Object%20Reference))
  (Game|Damage|ApplyDamage OtherActor (Variables|Default|GetMaxHealth) 0 0))

(fn ConstructionScript)