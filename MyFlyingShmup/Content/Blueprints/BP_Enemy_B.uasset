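; BP_Enemy_B is a turret-style enemy that faces the player and fires bullets on a timer.
; After running the parent BeginPlay, a looping timer spawns a BP_EnemyBullet at the Scene component's location every second.
; Each Tick, the Cube rotates to the look-at yaw toward the player pawn, with pitch and roll held at zero.
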(event Custom|ShootBullet
  (Game|SpawnActorfromClass "/Game/Blueprints/BP_EnemyBullet.BP_EnemyBullet_C" (Math|Transform|MakeTransform (.location (Transformation|GetWorldTransform (Variables|Default|GetScene))) "0, 0, 0" "1.000000,1.000000,1.000000") "AlwaysSpawn" "MultiplyWithRoot" 0 0))

(event EventBeginPlay
  (|CallParentFunction)
  (Utilities|Time|SetTimerbyEvent (delegate Custom|ShootBullet) 1.0 true))

(event EventTick
  (params (DeltaSeconds :type Float%20%28single-precision%29))
  (Transformation|SetWorldRotation (Variables|Default|GetCube) (Math|Rotator|MakeRotator 0.0 0.0 (.yaw (Math|Rotator|FindLookatRotation (Transformation|GetActorLocation) (Transformation|GetActorLocation (Game|Player|GetPlayerPawn 0))))) false false))

(fn ConstructionScript)