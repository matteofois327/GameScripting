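; BP_EnemyBoss1 is a boss enemy that moves itself into the play area, then moves from side to side.
; On BeginPlay, after the parent logic, an entry timeline slides it along negative X from its spawn location.
; When that finishes, it re-captures its location and a slowed timeline drives the Y offset.
; Both moves use swept location updates scaled from timeline curves.
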(event Custom|EnterPlayArea
  (Variables|Default|SetInitialLocation (Transformation|GetActorLocation))
  (bind _x_offset (Timeline|TL_EnterPlayArea PlayFromStart)
    (:Update
      (Transformation|SetActorLocation (+ (Variables|Default|GetInitialLocation) (Math|Vector|MakeVector (* _x_offset -1e+03) 0.0 0.0)) true false))
    (:Finished
      (CallFunction|MoveSidetoSide))))

(event Custom|MoveSideToSide
  (Variables|Default|SetInitialLocation (Transformation|GetActorLocation))
  (Components|Timeline|SetPlayRate (Variables|Default|GetTL_MoveSideToSide) 0.05)
  (bind _y_value (Timeline|TL_MoveSideToSide PlayFromStart)
    (:Update
      (Transformation|SetActorLocation (+ (Variables|Default|GetInitialLocation) (Math|Vector|MakeVector 0.0 (* _y_value 3e+03) 0.0)) true false))))

(event EventBeginPlay
  (|CallParentFunction)
  (CallFunction|EnterPlayArea))

(fn ConstructionScript
  (|CallParentFunction))